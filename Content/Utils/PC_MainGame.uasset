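; Player controller for a timed bubble tea order game, driving the BP_Comptoir counter actor and the menu and HUD widgets.
; LaunchGame and RetryGame start rounds, and EndGame disables input and ends the counter's game.
; Left, Up and Right pick ingredients step by step, Down resets, and Q/S/D/F send the order to one of four indices after four picks.
; AddScore awards clamped, streak-based points to the HUD.
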(event Custom|RetryGame
  ;[0.15 0.1222 0.05161 0.5] Begin
  (Variables|Default|SetScore 0)
  (CallFunction|ResetCommand)
  (Default|StartTimer (Variables|Default|GetMainGameWidget))
  (Input|EnableInput 0)
  (Default|LaunchGame (stale Custom|LaunchGame _output_get))
  (Default|UpdateScore (Variables|Default|GetMainGameWidget) (Variables|Default|GetScore)))

(event Custom|LaunchGame
  ;[0.15 0.1222 0.05161 0.5] Begin
  (Utilities|IsValid (Variables|Default|GetComptoir)
    (:Is%20Valid
      (CallFunction|AddMainGameWidget)
      (Variables|Default|SetScore 0)
      (CallFunction|ResetCommand))
    (:Is%20Not%20Valid
      (bind _returnvalue (Actor|GetActorOfClass "/Game/Comptoir/BP_Comptoir.BP_Comptoir_C"))
      (bind _output_get (Variables|Default|SetComptoir _returnvalue))
      (CallFunction|AddMainGameWidget)))
  (Default|StartTimer (Variables|Default|GetMainGameWidget))
  (Input|EnableInput 0)
  (Default|LaunchGame _output_get)
  (Default|UpdateScore (Variables|Default|GetMainGameWidget) (Variables|Default|GetScore)))

(event Custom|EndGame
  (Input|DisableInput 0)
  (Default|EndGame (Variables|Default|GetComptoir)))

(event EventBeginPlay
  ;[0.15 0.1222 0.05161 0.5] Begin
  (bind _returnvalue (UserInterface|CreateWidget "/Game/UI/W_MainMenu.W_MainMenu_C"))
  (UserInterface|Viewport|AddtoViewport _returnvalue 0)
  (Input|DisableInput 0))

(event Input|KeyboardEvents|Right
  (params (Key :type Key%20Structure :default "None"))
  ;[0.005285 0.15 0.02454 0.5] Inputs
  (:Pressed
    (Default|ChooseElement (Variables|Default|GetComptoir) 2 (Variables|Default|GetCountChoices))
    (Math|Integer|IncrementInt (Variables|Default|GetCountChoices)
      (:%20%20
        (Default|UpdateSelection (Variables|Default|GetComptoir) (Variables|Default|GetCountChoices))))))

(event Input|KeyboardEvents|Down
  (params (Key :type Key%20Structure :default "None"))
  ;[0.005285 0.15 0.02454 0.5] Inputs
  (:Pressed
    (CallFunction|ResetCommand)))

(event Input|KeyboardEvents|Left
  (params (Key :type Key%20Structure :default "None"))
  ;[0.005285 0.15 0.02454 0.5] Inputs
  (:Pressed
    (Default|ChooseElement (Variables|Default|GetComptoir) 0 (Variables|Default|GetCountChoices))
    (Math|Integer|IncrementInt (Variables|Default|GetCountChoices)
      (:%20%20
        (Default|UpdateSelection (Variables|Default|GetComptoir) (Variables|Default|GetCountChoices))))))

(event Input|KeyboardEvents|Q
  (params (Key :type Key%20Structure :default "None"))
  ;[0.005285 0.15 0.02454 0.5] Inputs
  (:Pressed
    (if (>= (Variables|Default|GetCountChoices) 4)
      (Default|SendCommand (Variables|Default|GetComptoir)))))

(event Input|KeyboardEvents|S
  (params (Key :type Key%20Structure :default "None"))
  ;[0.005285 0.15 0.02454 0.5] Inputs
  (:Pressed
    (if (>= (Variables|Default|GetCountChoices) 4)
      (Default|SendCommand (Variables|Default|GetComptoir) 1))))

(event Input|KeyboardEvents|D
  (params (Key :type Key%20Structure :default "None"))
  ;[0.005285 0.15 0.02454 0.5] Inputs
  (:Pressed
    (if (>= (Variables|Default|GetCountChoices) 4)
      (Default|SendCommand (Variables|Default|GetComptoir) 2))))

(event Input|KeyboardEvents|F
  (params (Key :type Key%20Structure :default "None"))
  ;[0.005285 0.15 0.02454 0.5] Inputs
  (:Pressed
    (if (>= (Variables|Default|GetCountChoices) 4)
      (Default|SendCommand (Variables|Default|GetComptoir) 3))))

(event Input|KeyboardEvents|Up
  (params (Key :type Key%20Structure :default "None"))
  ;[0.005285 0.15 0.02454 0.5] Inputs
  (:Pressed
    (Default|ChooseElement (Variables|Default|GetComptoir) 1 (Variables|Default|GetCountChoices))
    (Math|Integer|IncrementInt (Variables|Default|GetCountChoices)
      (:%20%20
        (Default|UpdateSelection (Variables|Default|GetComptoir) (Variables|Default|GetCountChoices))))))

(fn ConstructionScript)

(fn ResetCommand
  (bind _comptoir (Variables|Default|GetComptoir))
  (Variables|Default|SetCountChoices 0)
  (Default|SetBubbleTeaVisible _comptoir false)
  (Default|UpdateSelection _comptoir (Variables|Default|GetCountChoices)))

(fn AddScore
  (params (Streak :type Integer))
  (bind _returnvalue (Math|Integer|Clamp(Integer) Streak 1 4))
  (if (== _returnvalue 3)
    (bind _output_get (Variables|Default|SetScore (+ (Variables|Default|GetScore) 2)))
    (else
      (Variables|Default|SetScore (+ (Variables|Default|GetScore) _returnvalue))))
  (Default|UpdateScore (Variables|Default|GetMainGameWidget) _output_get))

(fn AddMainGameWidget
  (bind _returnvalue (UserInterface|CreateWidget "/Game/UI/W_MainGame.W_MainGame_C"))
  (UserInterface|Viewport|AddtoViewport _returnvalue 0)
  (Variables|Default|SetMainGameWidget _returnvalue))

(fn AddStreak
  (params (Param :type Integer))
  (Default|UpdateStreak (Variables|Default|GetMainGameWidget) Param))