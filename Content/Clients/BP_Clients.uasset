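; BP_Clients is a client actor that carries a randomly generated order and a countdown to despawn.
; The construction script calls GenerateCommand, which fills the Command array with four random integers.
; From BeginPlay, TimerLoop re-calls itself after each one-second delay, decrementing TimerBeforeDespawn until it sets IsTimerFinish.
; The Blueprint only raises that flag and does not destroy the actor itself.
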(event Custom|TimerLoop
  (Utilities|FlowControl|Delay 1.0)
  (bind _result (Math|Float|DecrementFloat (Variables|Default|GetTimerBeforeDespawn))
    (:%20%20
      (if (<= _result 0.0)
        (Variables|Default|SetIsTimerFinish true)
        (else
          (Variables|Default|SetIsTimerFinish false)
          (CallFunction|TimerLoop))))))

(event EventBeginPlay
  (CallFunction|TimerLoop))

(event Collision|EventActorBeginOverlap
  (params (OtherActor :type Actor%20Object%20Reference)))

(event EventTick
  (params (DeltaSeconds :type Float%20%28single-precision%29)))

(fn ConstructionScript
  (CallFunction|GenerateCommand))

(fn GenerateCommand
  (bind _returnvalue (Math|Random|RandomInteger 2))
  (bind _output_get (Variables|Default|SetCommand (Utilities|Array|MakeArray (Math|Random|RandomInteger 3) _returnvalue _returnvalue _returnvalue))))