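; Bubble tea shop client that shows a drink order and a world-widget countdown.
; A looping one-second timer updates the mm:ss display and plays a random voice sound at five seconds left.
; On timeout it resets the BP_Comptoir streak, hides, then asks the Comptoir for a new order after a random short delay.
; It also provides random four-part order generation and per-part drink material setup.
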(event Custom|StartTimer
  (params (TimerLengthSeconds :type Integer))
  ;[0.2948 0.03159 0.09501 0.5] Timer
  (Rendering|SetActorHiddenInGame false)
  (Variables|Default|SetWaitingCommand true)
  (bind _output_get (Variables|Default|SetInitialTime TimerLengthSeconds))
  (Variables|Default|SetTime _output_get)
  (bind _returnvalue (Utilities|Time|SetTimerbyEvent (delegate Custom|Delta1Second) 1.0 true))
  (Variables|Default|SetTimer _returnvalue)
  (Rendering|Components|TextRender|SetText (Variables|/Game/UI/W_ClientTimer.W_ClientTimer_C|GetTimer_Text (Variables|Default|GetTimerWidget)) (Utilities|Text|FormatText "{m}:{s}" (Utilities|Text|ToText(Integer) (/ (Variables|Default|GetTime) 60) false false 2 2) (Utilities|Text|ToText(Integer) (Math|Integer|%(Integer) (Variables|Default|GetTime) 60) false false 2 2)))
  (CallFunction|UpdateClientHappiness (Variables|Default|GetTime))
  (if (and (<= (Variables|Default|GetTime) 0) (Variables|Default|GetWaitingCommand))
    (bind _returnvalue_2 (Actor|GetActorOfClass "/Game/Comptoir/BP_Comptoir.BP_Comptoir_C"))
    (bind _output_get_2 (Variables|/Game/Comptoir/BP_Comptoir.BP_Comptoir_C|SetStreakCounter _returnvalue_2 0))
    (Default|AddStreak (Variables|/Game/Comptoir/BP_Comptoir.BP_Comptoir_C|Get%20PlayerRef _returnvalue_2) _output_get_2)
    (CallFunction|StopTimer)
    (CallFunction|ClientOut)))

(event Custom|ClientOut
  ;[0.2948 0.03159 0.09501 0.5] Timer
  (Rendering|SetActorHiddenInGame true)
  (Utilities|Time|SetTimerbyEvent (delegate Custom|NewCommand) (Math|Conversions|ToFloat(Integer) (Math|Random|RandomIntegerinRange 2 5)))
  (Variables|Default|SetWaitingCommand false))

(event Custom|Delta1Second
  ;[0.2948 0.03159 0.09501 0.5] Timer
  (Variables|Default|SetTime (- (Variables|Default|GetTime) 1))
  (Rendering|Components|TextRender|SetText (Variables|/Game/UI/W_ClientTimer.W_ClientTimer_C|GetTimer_Text (Variables|Default|GetTimerWidget)) (Utilities|Text|FormatText "{m}:{s}" (Utilities|Text|ToText(Integer) (/ (Variables|Default|GetTime) 60) false false 2 2) (Utilities|Text|ToText(Integer) (Math|Integer|%(Integer) (Variables|Default|GetTime) 60) false false 2 2)))
  (CallFunction|UpdateClientHappiness (Variables|Default|GetTime))
  (if (and (<= (Variables|Default|GetTime) 0) (Variables|Default|GetWaitingCommand))
    (bind _returnvalue (Actor|GetActorOfClass "/Game/Comptoir/BP_Comptoir.BP_Comptoir_C"))
    (bind _output_get (Variables|/Game/Comptoir/BP_Comptoir.BP_Comptoir_C|SetStreakCounter _returnvalue 0))
    (Default|AddStreak (Variables|/Game/Comptoir/BP_Comptoir.BP_Comptoir_C|Get%20PlayerRef _returnvalue) _output_get)
    (CallFunction|StopTimer)
    (CallFunction|ClientOut)))

(event Custom|PauseTimer
  ;[0.2948 0.03159 0.09501 0.5] Timer
  (Utilities|Time|PauseTimerbyHandle (Variables|Default|GetTimer)))

(event Custom|ResumeTimer
  ;[0.2948 0.03159 0.09501 0.5] Timer
  (Utilities|Time|UnpauseTimerbyHandle (Variables|Default|GetTimer)))

(event Custom|StopTimer
  ;[0.2948 0.03159 0.09501 0.5] Timer
  (Utilities|Time|ClearandInvalidateTimerbyHandle (Variables|Default|GetTimer))
  (Audio|PlaySound2D "/Game/Sound/Sounds_FX/Client_qui_part/SFX_Leave.SFX_Leave" 0.7 0.7 0.0 0 0))

(event Custom|NewCommand
  ;[0.2948 0.03159 0.09501 0.5] Timer
  (Default|GenerateNewCommandforClient (Variables|Default|GetComptoir) self))

(event EventBeginPlay
  (bind _asw_client_timer (Utilities|Casting|CastToW_ClientTimer (UserInterface|GetWidget (Variables|Default|GetTimerWidgetWorld))))
  (Variables|Default|SetTimerWidget _asw_client_timer))

(event Collision|EventActorBeginOverlap
  (params (OtherActor :type Actor%20Object%20Reference)))

(event EventTick
  (params (DeltaSeconds :type Float%20%28single-precision%29)))

(fn ConstructionScript)

(fn SetBubbleTea
  (params (Cup :type Material%20Instance%20Object%20Reference) (Tapioca :type Material%20Instance%20Object%20Reference) (Liquid :type Material%20Instance%20Object%20Reference) (Topping :type Material%20Instance%20Object%20Reference))
  (Rendering|Material|SetMaterial (Variables|Default|GetCup) 0 Cup)
  (Rendering|Material|SetMaterial (Variables|Default|GetBubbles) 0 Tapioca)
  (Rendering|Material|SetMaterial (Variables|Default|GetLiquid) 0 Liquid)
  (Rendering|Material|SetMaterial (Variables|Default|GetTopping) 0 Topping))

(fn GenerateNewCommand
  (bind _output_get (Variables|Default|SetCommand (Utilities|Struct|MakeS_Command (Math|Random|RandomInteger 3) (Math|Random|RandomInteger 3) (Math|Random|RandomInteger 3) (Math|Random|RandomInteger 3))))
  (return _output_get))

(fn UpdateClientHappiness
  (params (Timer :type Integer))
  (if (== Timer 5)
    (Audio|PlaySound2D (Utilities|Array|Get(acopy) (Variables|Default|GetSoundListHappy) (Math|Random|RandomInteger 7)) 0.7 0.7 0.0 0 0)))