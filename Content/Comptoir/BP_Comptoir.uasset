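; Bubble tea counter that runs the drink-making game: clients order random drinks on a timer and the player's assembled drink is checked against their orders.
; The construction script fills four selection displays with three material variants each for cup, tapioca, liquid and topping.
; ChooseElement updates the drink's visuals, sounds and Niagara effects, picking FX colors by material name.
; SendCommand compares all four choices to the client's order, updating score and streak.
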(event Custom|LaunchGame
  (Development|SetHiddeninGame (Variables|Default|GetClientsScene) false true)
  (CallFunction|UpdateSelection)
  (for _array_element (Variables|Default|GetClients)
    (CallFunction|GenerateNewCommandforClient _array_element)))

(event EventBeginPlay
  (bind _aspc_main_game (Utilities|Casting|CastToPC_MainGame (Game|GetPlayerController 0)))
  (Variables|Default|Set%20PlayerRef _aspc_main_game)
  (bind _asbp_bubble_tea (Utilities|Casting|CastToBP_BubbleTea (Variables|/Script/Engine.ChildActorComponent|GetChildActor (Variables|Default|GetBubbleTeaActor))))
  (Variables|Default|SetBubbleTeaRef _asbp_bubble_tea)
  (CallFunction|SetBubbleTeaVisible false)
  (bind _asbp_bubble_client (Utilities|Casting|CastToBP_BubbleClient (Variables|/Script/Engine.ChildActorComponent|GetChildActor (Variables|Default|GetClient0))))
  (Utilities|Array|Add (Variables|Default|GetClients) _asbp_bubble_client)
  (bind _asbp_bubble_client_2 (Utilities|Casting|CastToBP_BubbleClient (Variables|/Script/Engine.ChildActorComponent|GetChildActor (Variables|Default|GetClient1))))
  (Utilities|Array|Add (Variables|Default|GetClients) _asbp_bubble_client_2)
  (bind _asbp_bubble_client_3 (Utilities|Casting|CastToBP_BubbleClient (Variables|/Script/Engine.ChildActorComponent|GetChildActor (Variables|Default|GetClient2))))
  (Utilities|Array|Add (Variables|Default|GetClients) _asbp_bubble_client_3)
  (bind _asbp_bubble_client_4 (Utilities|Casting|CastToBP_BubbleClient (Variables|/Script/Engine.ChildActorComponent|GetChildActor (Variables|Default|GetClient3))))
  (Utilities|Array|Add (Variables|Default|GetClients) _asbp_bubble_client_4)
  (for _array_element (Variables|Default|GetClients)
    (Variables|/Game/Clients/BP_BubbleClient.BP_BubbleClient_C|SetComptoir _array_element self))
  (Development|SetHiddeninGame (Variables|Default|GetClientsScene) true true))

(fn ConstructionScript
  (CallFunction|InitSelection (Variables|Default|GetCupSelection) "/Game/Assets/Props/Gobelet/SM_Gobelet.SM_Gobelet" (Variables|Colors|GetCupColor))
  (CallFunction|InitSelection (Variables|Default|GetTapiocaSelection) "/Game/Assets/Props/TapiocaVisuel/SM_TapiocaVisuel.SM_TapiocaVisuel" (Variables|Colors|GetTapiocaColor))
  (CallFunction|InitSelection (Variables|Default|GetLiquidSelection) "/Game/Assets/Props/LiquideVisuel/SM_LiquideVisuel.SM_LiquideVisuel" (Variables|Colors|GetLiquidColor))
  (CallFunction|InitSelection (Variables|Default|GetToppingSelection) "/Game/Assets/Props/ToppingVisuel/SM_ToppingVisuel.SM_ToppingVisuel" (Variables|Colors|GetToppingColor)))

(fn InitSelection
  (params (SelectionActor :type Child%20Actor%20Component%20Object%20Reference) (Mesh :type Static%20Mesh%20Object%20Reference) (Colors :type Array%20of%20Material%20Instance%20Object%20References))
  (bind _asbp_selection (Utilities|Casting|CastToBP_Selection (Variables|/Script/Engine.ChildActorComponent|GetChildActor SelectionActor)))
  (CallFunction|SetSelectionMeshMaterial (Variables|/Game/Comptoir/BP_Selection.BP_Selection_C|GetStaticMeshLeft _asbp_selection) Mesh (Utilities|Array|Get(acopy) Colors))
  (CallFunction|SetSelectionMeshMaterial (Variables|/Game/Comptoir/BP_Selection.BP_Selection_C|GetStaticMeshUp _asbp_selection) Mesh (Utilities|Array|Get(acopy) Colors 1))
  (CallFunction|SetSelectionMeshMaterial (Variables|/Game/Comptoir/BP_Selection.BP_Selection_C|GetStaticMeshRight _asbp_selection) Mesh (Utilities|Array|Get(acopy) Colors 2)))

(fn SetSelectionMeshMaterial
  (params (MeshSelect :type Static%20Mesh%20Component%20Object%20Reference) (Mesh :type Static%20Mesh%20Object%20Reference) (Material :type Material%20Instance%20Object%20Reference))
  (Components|StaticMesh|SetStaticMesh MeshSelect Mesh)
  (Rendering|Material|SetMaterial MeshSelect 0 Material))

(fn GenerateNewCommandforClient
  (params (Client :type BP%20Bubble%20Client%20Object%20Reference))
  (bind _newcommand (Default|GenerateNewCommand Client))
  (Default|SetBubbleTea Client (Utilities|Array|Get(acopy) (Variables|Colors|GetCupColor) (.cup _newcommand)) (Utilities|Array|Get(acopy) (Variables|Colors|GetTapiocaColor) (.tapioca _newcommand)) (Utilities|Array|Get(acopy) (Variables|Colors|GetLiquidColor) (.liquid _newcommand)) (Utilities|Array|Get(acopy) (Variables|Colors|GetToppingColor) (.topping _newcommand)))
  (Default|StartTimer Client 20))

(fn ChooseElement
  (params (SelectedValue :type Integer) (CountChoices :type Integer))
  (bind _bubbletea (Variables|Default|GetBubbleTea))
  (switch int CountChoices
    (:0
      (Utilities|Struct|SetmembersinS_Command _bubbletea SelectedValue))
    (:1
      (Utilities|Struct|SetmembersinS_Command _bubbletea SelectedValue))
    (:2
      (Utilities|Struct|SetmembersinS_Command _bubbletea SelectedValue))
    (:3
      (Utilities|Struct|SetmembersinS_Command _bubbletea SelectedValue)))
  (CallFunction|UpdateBubbleTea CountChoices))

(fn UpdateBubbleTea
  (params (Selection :type Integer))
  (bind _bubbletea (Variables|Default|GetBubbleTea))
  (bind _liquidcolor (Variables|Colors|GetLiquidColor))
  (bind _bubbletearef (Variables|Default|GetBubbleTeaRef))
  (bind _bubbletearef_2 (Variables|Default|GetBubbleTeaRef))
  (bind _bubbletearef_3 (Variables|Default|GetBubbleTeaRef))
  (bind _tapiocacolor (Variables|Colors|GetTapiocaColor))
  (bind _bubbletea_2 (Variables|Default|GetBubbleTea))
  (bind _bubbletearef_4 (Variables|Default|GetBubbleTeaRef))
  (bind _output (Utilities|Array|Get(acopy) _liquidcolor (.liquid _bubbletea)))
  (bind _output_2 (Utilities|Array|Get(acopy) _tapiocacolor (.tapioca _bubbletea_2)))
  (bind _bubbles (Variables|/Game/Comptoir/Utils/BP_BubbleTea.BP_BubbleTea_C|GetBubbles _bubbletearef_2))
  (bind _cup (Variables|/Game/Comptoir/Utils/BP_BubbleTea.BP_BubbleTea_C|GetCup _bubbletearef_3))
  (bind _liquid (Variables|/Game/Comptoir/Utils/BP_BubbleTea.BP_BubbleTea_C|GetLiquid _bubbletearef))
  (bind _topping (Variables|/Game/Comptoir/Utils/BP_BubbleTea.BP_BubbleTea_C|GetTopping _bubbletearef_4))
  (switch int Selection
    (:0
      (Rendering|SetVisibility _cup true false)
      (Rendering|Material|SetMaterial _cup 0 (Utilities|Array|Get(acopy) (Variables|Colors|GetCupColor) (.cup (Variables|Default|GetBubbleTea))))
      (Audio|PlaySound2D (Utilities|Array|Get(acopy) (Variables|Sounds|GetSoundForCup) (Math|Random|RandomInteger 7)) 0.7 0.7 0.0 0 0))
    (:1
      (Rendering|SetVisibility _bubbles true false)
      (Rendering|Material|SetMaterial _bubbles 0 _output_2)
      (CallFunction|UpdateFXTapiocca (Utilities|GetObjectName _output_2)))
    (:2
      (Rendering|SetVisibility _liquid true false)
      (Rendering|Material|SetMaterial _liquid 0 _output)
      (CallFunction|UpdateFXLiquid (Utilities|GetObjectName _output)))
    (:3
      (Rendering|SetVisibility _topping true false)
      (Rendering|Material|SetMaterial _topping 0 (Utilities|Array|Get(acopy) (Variables|Colors|GetToppingColor) (.topping (Variables|Default|GetBubbleTea))))
      (Audio|PlaySound2D (Utilities|Array|Get(acopy) (Variables|Sounds|GetSoundForTopping) (Math|Random|RandomInteger 5)) 0.7 0.7 0.0 0 0))))

(fn UpdateSelection
  (params (Selection :type Integer))
  (for (_array_element _array_index) (Utilities|Array|MakeArray (Variables|Default|GetCupSelection) (Variables|Default|GetTapiocaSelection) (Variables|Default|GetLiquidSelection) (Variables|Default|GetToppingSelection))
    (bind _asbp_selection (Utilities|Casting|CastToBP_Selection (Variables|/Script/Engine.ChildActorComponent|GetChildActor _array_element)))
    (Default|SetSelectVisible _asbp_selection (== _array_index Selection))))

(fn UpdateFXTapiocca
  (params (Name :type String))
  (Audio|PlaySound2D (Utilities|Array|Get(acopy) (Variables|Sounds|GetSoundForTapioca) (Math|Random|RandomInteger 7)) 0.7 0.7 0.0 0 0)
  (bind _returnvalue (Niagara|SpawnSystematLocation "/Game/FX/Niagara-System/NS_Tapioca.NS_Tapioca" "413.000000,10.000000,150.000000" "0, 0, 0" "1.000000,1.000000,1.000000" true true "AutoRelease"))
  (if (Utilities|Enum|Equal(Enum) Name "M_TapiocaRed")
    (Effects|Components|ParticleSystem|SetColorParameter _returnvalue "TapiocaFX" (Utilities|Struct|MakeLinearColor 1.0 0.0 0.0 0.0))
    (elif (Utilities|Enum|Equal(Enum) Name "M_TapiocaWhite")
      (Effects|Components|ParticleSystem|SetColorParameter _returnvalue "TapiocaFX" (Utilities|Struct|MakeLinearColor 0.922 0.902412 0.906104 1.0))
      (elif (Utilities|Enum|Equal(Enum) Name "M_TapiocaYellow")
        (Effects|Components|ParticleSystem|SetColorParameter _returnvalue "TapiocaFX" (Utilities|Struct|MakeLinearColor 1.0 0.618826 0.0 1.0))))))

(fn UpdateFXLiquid
  (params (Name :type String))
  (Audio|PlaySound2D (Utilities|Array|Get(acopy) (Variables|Sounds|GetSoundForLiquid) (Math|Random|RandomInteger 7)) 0.7 0.7 0.0 0 0)
  (bind _returnvalue (Niagara|SpawnSystematLocation "/Game/FX/Niagara_System/NS_Liquid.NS_Liquid" "410.000000,129.000000,230.000000" "0, 0, 0" "1.000000,1.000000,1.000000" true true "AutoRelease"))
  (if (Utilities|Enum|Equal(Enum) Name "M_LiquidGreen")
    (Effects|Components|ParticleSystem|SetColorParameter _returnvalue "ColorRed" (Utilities|Struct|MakeLinearColor 0.083984 1.0 0.0 1.0))
    (elif (Utilities|Enum|Equal(Enum) Name "M_LiquidGray")
      (Effects|Components|ParticleSystem|SetColorParameter _returnvalue "ColorRed" (Utilities|Struct|MakeLinearColor 0.5 0.5 0.5 0.0))
      (elif (Utilities|Enum|Equal(Enum) Name "M_LiquidBlue")
        (Effects|Components|ParticleSystem|SetColorParameter _returnvalue "ColorRed" (Utilities|Struct|MakeLinearColor 0.007296 1.0 1.0 0.0))))))

(fn SetBubbleTeaVisible
  (params (Visible :type Boolean))
  (Rendering|SetVisibility (Variables|/Game/Comptoir/Utils/BP_BubbleTea.BP_BubbleTea_C|GetCup (Variables|Default|GetBubbleTeaRef)) Visible false))

(fn SendCommand
  (params (ClientNumber :type Integer))
  (bind _bubbletea (Variables|Default|GetBubbleTea))
  (bind (_cup _tapioca _liquid _topping) (Utilities|Struct|BreakS_Command _bubbletea))
  (bind _output_get (LocalVariables|SetClient (Utilities|Array|Get(acopy) (Variables|Default|GetClients) ClientNumber)))
  (if (Variables|/Game/Clients/BP_BubbleClient.BP_BubbleClient_C|GetWaitingCommand _output_get)
    (if (Utilities|Array|Identical (Utilities|Array|MakeArray (.Cup (Utilities|Struct|BreakS_Command (Variables|/Game/Clients/BP_BubbleClient.BP_BubbleClient_C|GetCommand _output_get))) (.Tapioca (Utilities|Struct|BreakS_Command (Variables|/Game/Clients/BP_BubbleClient.BP_BubbleClient_C|GetCommand _output_get))) (.Liquid (Utilities|Struct|BreakS_Command (Variables|/Game/Clients/BP_BubbleClient.BP_BubbleClient_C|GetCommand _output_get))) (.Topping (Utilities|Struct|BreakS_Command (Variables|/Game/Clients/BP_BubbleClient.BP_BubbleClient_C|GetCommand _output_get)))) (Utilities|Array|MakeArray _cup _tapioca _liquid _topping))
      (Audio|PlaySound2D "/Game/Sound/Sounds_FX/Win/Sound_Win.Sound_Win" 0.7 0.7 0.0 0 0)
      (Niagara|SpawnSystematLocation "/Game/FX/Niagara_System/NS_Correct.NS_Correct" (Transformation|GetActorLocation _output_get) "0, 0, 0" "1.000000,1.000000,1.000000" true true "AutoRelease")
      (Default|AddScore (Variables|Default|Get%20PlayerRef))
      (Math|Integer|IncrementInt (LocalVariables|GetStreakCounter)
        (:%20%20
          _))
      (else
        (Audio|PlaySound2D "/Game/Sound/Sounds_FX/Lose/Sound_Lose.Sound_Lose" 0.7 0.7 0.0 0 0)
        (Niagara|SpawnSystematLocation "/Game/FX/Niagara_System/NS_Incorrect.NS_Incorrect" (Transformation|GetActorLocation _output_get) "0, 0, 0" "1.000000,1.000000,1.000000" true true "AutoRelease")
        (LocalVariables|SetStreakCounter 0)))
    (Default|ResetCommand (Variables|Default|Get%20PlayerRef))
    (Default|ClientOut (LocalVariables|GetClient))))